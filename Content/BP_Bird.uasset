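; Player bird for a Flappy Bird-style game: loads the high score, then shows the main menu with the game paused.
; Tick pushes the physics cube forward and caps its height; touch or Space adds an upward impulse with sound and squash timeline.
; Hitting anything except a BP_BouncyPipe records the score and reloads the level.
; UpdateLeaderboard inserts positive scores into a ranked, capped BP_SaveData list, flagging the new entry.
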(event OnComponentHit(Cube)
  (params (HitComponent :type Primitive%20Component%20Object%20Reference) (OtherActor :type Actor%20Object%20Reference) (OtherComp :type Primitive%20Component%20Object%20Reference) (NormalImpulse :type Vector :default "0, 0, 0") (Hit :type Hit%20Result%20Structure%20%28by%20ref%29))
  (Utilities|Casting|CastToBP_BouncyPipe OtherActor
    (:CastFailed
      (CallFunction|UpdateLeaderboard (Variables|Default|GetScore))
      (bind _returnvalue (Game|GetCurrentLevelName true))
      (Game|OpenLevel(byName) (Utilities|String|StringToName _returnvalue)))))

(event EventBeginPlay
  (Utilities|FlowControl|Sequence
    (:then_0
      (bind _returnvalue (SaveGame|DoesSaveGameExist "Leaderboard_Final_Test_1"))
      (if _returnvalue
        (bind _returnvalue_2 (SaveGame|LoadGamefromSlot "Leaderboard_Final_Test_1"))
        (bind _asbp_save_data (Utilities|Casting|CastToBP_SaveData _returnvalue_2))
        (Variables|Default|SetHighScore (.Score (Utilities|Struct|BreakS_ScoreEntry (Utilities|Array|Get(acopy) (Variables|/Game/BP_SaveData.BP_SaveData_C|GetLeaderboardList _asbp_save_data)))))
        (else
          (Variables|Default|SetHighScore 0))))
    (:then_1
      (bind _returnvalue_3 (UserInterface|CreateWidget "/Game/WBP_MainMenu.WBP_MainMenu_C"))
      (UserInterface|Viewport|AddtoViewport _returnvalue_3 0)
      (Game|SetGamePaused true)
      (Input|SetInputModeUIOnly (Game|GetPlayerController 0) 0 "DoNotLock" false))))

(event Collision|EventActorBeginOverlap
  (params (OtherActor :type Actor%20Object%20Reference)))

(event EventTick
  (params (DeltaSeconds :type Float%20%28single-precision%29))
  (bind _returnvalue (Transformation|GetActorLocation))
  (Utilities|FlowControl|Sequence
    (:then_0
      (Physics|AddForce (Variables|Default|GetCube) "1000000.000000,0.000000,0.000000" "None" false))
    (:then_1
      (if (> (.z _returnvalue) 1.2e+03)
        (Transformation|SetActorLocation (Math|Vector|MakeVector (.x _returnvalue) (.y _returnvalue) 1e+03) false false)
        (bind _returnvalue_2 (Physics|GetPhysicsLinearVelocity (Variables|Default|GetCube) "None"))
        (Physics|SetPhysicsLinearVelocity (Variables|Default|GetCube) (Math|Vector|MakeVector (.x _returnvalue_2) 0.0 0.0) false "None")))))

(event Input|KeyboardEvents|SpaceBar
  (params (Key :type Key%20Structure :default "None"))
  (:Pressed
    (Audio|PlaySound2D "/Game/flysquishpopsound.flysquishpopsound" 1.0 1.0 0.0 0 0)
    (Physics|AddImpulse (Variables|Default|GetCube) "0.000000,0.000000,800.000000" "None" true)
    (bind _newtrack_0 (Timeline|FlapAnim PlayFromStart)
      (:Update
        (Transformation|SetWorldScale3D (Variables|Default|GetCube) (Math|Vector|MakeVector 1.0 1.0 _newtrack_0))))))

(event Input|TouchEvents|Touch1
  (params (Key :type Key%20Structure :default "None"))
  (:Pressed
    (Audio|PlaySound2D "/Game/flysquishpopsound.flysquishpopsound" 1.0 1.0 0.0 0 0)
    (Physics|AddImpulse (Variables|Default|GetCube) "0.000000,0.000000,800.000000" "None" true)
    (bind _newtrack_0 (Timeline|FlapAnim PlayFromStart)
      (:Update
        (Transformation|SetWorldScale3D (Variables|Default|GetCube) (Math|Vector|MakeVector 1.0 1.0 _newtrack_0))))))

(fn ConstructionScript)

(fn UpdateLeaderboard
  (params (NewScore :type Integer))
  (bind _s_scoreentry (Utilities|Struct|MakeS_ScoreEntry NewScore "You" true))
  (if (> NewScore 0)
    (bind _returnvalue (SaveGame|DoesSaveGameExist "Leaderboard_Final_Test_1"))
    (if _returnvalue
      (bind _returnvalue_2 (SaveGame|LoadGamefromSlot "Leaderboard_Final_Test_1"))
      (bind _asbp_save_data (Utilities|Casting|CastToBP_SaveData _returnvalue_2)
        (:then
          (for (_array_element _array_index) (Variables|/Game/BP_SaveData.BP_SaveData_C|GetLeaderboardList _asbp_save_data)
            (bind _structout (Utilities|Struct|SetmembersinS_ScoreEntry _array_element false))
            (Utilities|Array|SetArrayElem (Variables|/Game/BP_SaveData.BP_SaveData_C|GetLeaderboardList _asbp_save_data) _array_index _structout))
          (Variables|Default|SetFoundIndex -1)
          (bind (_array_element_2 _array_index_2) (Utilities|Array|ForEachLoopwithBreak (Variables|/Game/BP_SaveData.BP_SaveData_C|GetLeaderboardList _asbp_save_data) :!label _label)
            (:LoopBody
              (if (> NewScore (.Score (Utilities|Struct|BreakS_ScoreEntry _array_element_2)))
                (Variables|Default|SetFoundIndex _array_index_2)
                (goto _label Break)))
            (:Completed
              (if (>= (Variables|Default|GetFoundIndex) 0)
                (Utilities|Array|Insert (Variables|/Game/BP_SaveData.BP_SaveData_C|GetLeaderboardList _asbp_save_data) _s_scoreentry (Variables|Default|GetFoundIndex))
                (else
                  (Utilities|Array|Add (Variables|/Game/BP_SaveData.BP_SaveData_C|GetLeaderboardList _asbp_save_data) _s_scoreentry)))
              (if (> (Utilities|Array|Length (Variables|/Game/BP_SaveData.BP_SaveData_C|GetLeaderboardList _asbp_save_data)) 15)
                (Utilities|Array|Resize (Variables|/Game/BP_SaveData.BP_SaveData_C|GetLeaderboardList _asbp_save_data) 15))
              (SaveGame|SaveGametoSlot _asbp_save_data "Leaderboard_Final_Test_1"))))
        (:CastFailed
          (bind _returnvalue_3 (SaveGame|CreateSaveGameObject "/Game/BP_SaveData.BP_SaveData_C" :!label _label_2))
          (Utilities|Array|Add (Variables|/Game/BP_SaveData.BP_SaveData_C|GetLeaderboardList _returnvalue_3) _s_scoreentry)
          (SaveGame|SaveGametoSlot _returnvalue_3 "Leaderboard_Final_Test_1")))
      (else
        (goto _label_2)))))