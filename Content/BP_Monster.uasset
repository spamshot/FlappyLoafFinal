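; BP_Monster is a monster actor that advances along the world X axis at its MonsterSpeed.
; Each tick it moves forward by frame-scaled speed and sets its height to a fixed distance below the player pawn, tracking the player vertically.
; On BeginPlay, the ChompAnim timeline drives the JawHinge component's relative Z location to animate a chomping jaw.
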(event EventBeginPlay
  (bind _newtrack_0 (Timeline|ChompAnim Play)
    (:Update
      (Transformation|SetRelativeLocation (Variables|Default|GetJawHinge) (Math|Vector|MakeVector 0.0 0.0 _newtrack_0) false false))))

(event Collision|EventActorBeginOverlap
  (params (OtherActor :type Actor%20Object%20Reference)))

(event EventTick
  (params (DeltaSeconds :type Float%20%28single-precision%29))
  (Transformation|SetActorLocation (Math|Vector|MakeVector (+ (.x (Transformation|GetActorLocation)) (* (Variables|Default|GetMonsterSpeed) (Utilities|Time|GetWorldDeltaSeconds))) 0.0 (- (.z (Transformation|GetActorLocation (Game|Player|GetPlayerPawn 0))) 2e+02)) false false))

(fn ConstructionScript)