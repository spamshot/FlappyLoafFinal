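; Spawner actor that places pipe obstacles ahead of the player pawn at random heights, apparently for a Flappy Bird-style game.
; A looping timer started on BeginPlay projects a spawn point ahead along X and spawns only if it clears the last pipe's X by a minimum gap.
; The first pipe is BP_Pipe and every later one is BP_BouncyPipe, chosen by a running pipe count.
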(event Custom|SpawnPipe
  (bind _returnvalue (Game|Player|GetPlayerPawn 0))
  (bind _returnvalue_2 (Transformation|GetActorLocation _returnvalue))
  (bind _returnvalue_3 (+ (.x _returnvalue_2) 1.5e+03))
  (if (> _returnvalue_3 (+ (Variables|Default|GetLastPipeX) 2.1e+02))
    (Variables|Default|SetLastPipeX _returnvalue_3)
    (Math|Integer|IncrementInt (Variables|Default|GetPipeCount)
      (:%20%20
        (Game|SpawnActorfromClass (select (== (Variables|Default|GetPipeCount) 1) "/Game/BP_Pipe.BP_Pipe_C" "/Game/BP_BouncyPipe.BP_BouncyPipe_C") (Math|Transform|MakeTransform (Math|Vector|MakeVector _returnvalue_3 (.y _returnvalue_2) (Math|Random|RandomFloatinRange 0.0 8e+02)) "0, 0, 0" (Math|Vector|MakeVector 1.0 1.0 1.0)) "Undefined" "MultiplyWithRoot" 0 0)))))

(event EventBeginPlay
  (Utilities|Time|SetTimerbyEvent (delegate Custom|SpawnPipe) 2.5 true))

(event Collision|EventActorBeginOverlap
  (params (OtherActor :type Actor%20Object%20Reference)))

(event EventTick
  (params (DeltaSeconds :type Float%20%28single-precision%29)))

(fn ConstructionScript)